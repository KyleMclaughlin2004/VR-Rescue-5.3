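; Spline actor that carries a skeletal-mesh dummy toward the nacelle in a VR scene while the referenced BP_Drill is spinning.
; Tick advances the mesh along the spline, orienting it from the start tangent with fixed offsets.
; A Delay, rather than spline distance, flags nacelle arrival, which combines with a grabbed flag to set TakeOffAnchor.
; A sphere overlap with either VR pawn hand collider marks the dummy as overlapped.
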(event OnComponentBeginOverlap(Sphere)
  (params (OverlappedComponent :type Primitive%20Component%20Object%20Reference) (OtherActor :type Actor%20Object%20Reference) (OtherComp :type Primitive%20Component%20Object%20Reference) (OtherBodyIndex :type Integer) (bFromSweep :type Boolean) (SweepResult :type Hit%20Result%20Structure%20%28by%20ref%29))
  (bind _asvrpawn (Utilities|Casting|CastToVRPawn OtherActor))
  (if (or (== OtherComp (Variables|/Game/VRTemplate/Blueprints/VRPawn.VRPawn_C|GetRightHandCollider _asvrpawn)) (== (Variables|/Game/VRTemplate/Blueprints/VRPawn.VRPawn_C|GetLeftHandCollider _asvrpawn) OtherComp))
    (Variables|Default|SetOverlappedDummy true)))

(event EventBeginPlay
  (bind _returnvalue (Actor|GetActorOfClass "/Game/Equipment/BP_Drill.BP_Drill_C"))
  (Variables|Default|SetDrillRef _returnvalue))

(event EventTick
  (params (DeltaSeconds :type Float%20%28single-precision%29))
  (bind _spline (Variables|Default|GetSpline))
  (bind _returnvalue (Spline|GetTangentatDistanceAlongSpline _spline 0.0 "Local"))
  (bind _returnvalue_2 (Math|Conversions|ToVector(Float) (.z _returnvalue)))
  (bind _returnvalue_3 (Math|Conversions|ToVector(Float) (.x _returnvalue)))
  (bind _returnvalue_4 (Math|Rotator|MakeRotfromXZ _returnvalue_3 _returnvalue_2))
  (Utilities|FlowControl|Sequence
    (:then_0
      (if (Variables|Default|GetShouldGoToNacelle?)
        (if (Variables|/Game/Equipment/BP_Drill.BP_Drill_C|GetSpinning (Variables|Default|GetDrillRef))
          (Variables|Default|SetDistanceAlongSpline (+ (* DeltaSeconds (Variables|Default|GetSplineSpeed)) (Variables|Default|GetDistanceAlongSpline)))
          (Transformation|SetRelativeLocation (Variables|Default|GetSkeletalMesh) (Spline|GetLocationatDistanceAlongSpline (Variables|Default|GetSpline) (Variables|Default|GetDistanceAlongSpline) "Local") false false)
          (Transformation|SetRelativeRotation (Variables|Default|GetSkeletalMesh) (Math|Rotator|MakeRotator (+ (.roll _returnvalue_4) 9e+01) 9e+01 (- (.yaw _returnvalue_4) 55.0)) false false)
          (Utilities|FlowControl|Delay 4.0)
          (Variables|Default|SetReachedNacelle? true))))
    (:then_1
      (if (Variables|Default|GetReachedNacelle?)
        (if (Variables|Default|GetGrabbedDummy)
          (Variables|Default|SetTakeOffAnchor true))))))

(fn ConstructionScript)