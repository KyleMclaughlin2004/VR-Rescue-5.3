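; BP_PlayerClip is a physics-driven rope clip that the VR player attaches to themselves.
; Once Enabled, Tick runs a one-time release that zeroes velocity, shows the clip and rope, and turns on gravity and physics.
; Tick then polls its Sphere against the VRPawn's DrillDropPoint; on overlap it flags AttachedToPlayer and reveals the pawn's two carabiner meshes.
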(event EventTick
  (params (DeltaSeconds :type Float%20%28single-precision%29))
  (bind _ropeclipmesh (Variables|Default|GetRopeClipMesh))
  (bind _vr_pawn_ref (Variables|Default|GetVR%20Pawn%20Ref))
  (if (Variables|Default|GetEnabled)
    (if (not (Variables|Default|GetAttachedToPlayer))
      (Utilities|FlowControl|Sequence
        (:then_0
          (Utilities|FlowControl|DoOnce false
            (:Completed
              (Physics|SetEnableGravity _ropeclipmesh true)
              (Physics|SetPhysicsLinearVelocity _ropeclipmesh "0, 0, 0" false "None")
              (Class|PrimitiveComponent|SetPhysicsAngularVelocityinDegrees _ropeclipmesh "0, 0, 0" false "None")
              (Rendering|SetVisibility _ropeclipmesh true false)
              (Physics|SetSimulatePhysics _ropeclipmesh true))))
        (:then_1
          (if (Class|PrimitiveComponent|IsOverlappingComponent (Variables|Default|GetSphere) (Variables|/Game/VRTemplate/Blueprints/VRPawn.VRPawn_C|GetDrillDropPoint _vr_pawn_ref))
            (Variables|Default|SetAttachedToPlayer true)
            (Utilities|FlowControl|DoOnce false
              (:Completed
                (Rendering|SetVisibility (Variables|/Game/VRTemplate/Blueprints/VRPawn.VRPawn_C|GetCarabiner1 _vr_pawn_ref) true false)))))))))

(event EventBeginPlay
  (bind _returnvalue (Actor|GetActorOfClass "/Game/VRTemplate/Blueprints/VRPawn.VRPawn_C"))
  (Variables|Default|SetVR%20Pawn%20Ref _returnvalue))

(fn ConstructionScript)