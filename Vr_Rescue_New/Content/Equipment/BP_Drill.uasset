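; VR drill equipment that docks onto a rotor and plays a drilling sound while spinning in the player's hand.
; Tick scans both VR pawn hand colliders for the drill-tagged component and retriggers the sound through a delayed DoOnce reset.
; Overlapping a rope-attached BP_Rotor releases the grab, stops physics motion and gravity, and snaps the mesh to the DrillSocket position and yaw.
; Leaving the rotor restores gravity and clears the anchored state.
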(event OnComponentBeginOverlap(DrillCollider)
  (params (OverlappedComponent :type Primitive%20Component%20Object%20Reference) (OtherActor :type Actor%20Object%20Reference) (OtherComp :type Primitive%20Component%20Object%20Reference) (OtherBodyIndex :type Integer) (bFromSweep :type Boolean) (SweepResult :type Hit%20Result%20Structure%20%28by%20ref%29))
  (bind _drillmesh (Variables|Default|GetDrillMesh))
  (bind _asbp_rotor (Utilities|Casting|CastToBP_Rotor OtherActor))
  (if (Variables|/Game/Equipment/BP_Rotor.BP_Rotor_C|GetRopeAttached _asbp_rotor)
    (Utilities|FlowControl|DoOnce false
      (:Completed
        (Default|TryRelease (Variables|Default|GetGrabComponent))
        (Physics|SetEnableGravity _drillmesh false)
        (Physics|SetPhysicsLinearVelocity _drillmesh "0, 0, 0" false "None")
        (Class|PrimitiveComponent|SetPhysicsAngularVelocityinDegrees _drillmesh "0, 0, 0" false "None")
        (Transformation|SetWorldLocation _drillmesh (Transformation|GetSocketLocation (Variables|/Game/Equipment/BP_Rotor.BP_Rotor_C|GetRotorMesh _asbp_rotor) "DrillSocket") false false)
        (Transformation|SetWorldRotation _drillmesh (Math|Rotator|MakeRotator 0.0 0.0 (.Yaw (Math|Rotator|BreakRotator (Transformation|GetSocketRotation (Variables|/Game/Equipment/BP_Rotor.BP_Rotor_C|GetRotorMesh _asbp_rotor) "DrillSocket")))) false false)
        (Variables|Default|SetIsOnAnchor true)))))

(event OnComponentEndOverlap(DrillCollider)
  (params (OverlappedComponent :type Primitive%20Component%20Object%20Reference) (OtherActor :type Actor%20Object%20Reference) (OtherComp :type Primitive%20Component%20Object%20Reference) (OtherBodyIndex :type Integer))
  (bind _drillmesh (Variables|Default|GetDrillMesh))
  (Utilities|Casting|CastToBP_Rotor OtherActor)
  (Physics|SetEnableGravity (Variables|Default|GetDrillMesh) true)
  (Variables|Default|SetIsOnAnchor false)
  (Utilities|FlowControl|DoOnce false) ; enters at Reset
)

(event EventBeginPlay
  (bind _returnvalue (Actor|GetActorOfClass "/Game/VRTemplate/Blueprints/VRPawn.VRPawn_C"))
  (Variables|Default|SetVR%20Pawn%20Ref _returnvalue))

(event EventTick
  (params (DeltaSeconds :type Float%20%28single-precision%29))
  (bind _vr_pawn_ref (Variables|Default|GetVR%20Pawn%20Ref))
  (bind _righthandcollider (Variables|/Game/VRTemplate/Blueprints/VRPawn.VRPawn_C|GetRightHandCollider _vr_pawn_ref))
  (bind _lefthandcollider (Variables|/Game/VRTemplate/Blueprints/VRPawn.VRPawn_C|GetLeftHandCollider _vr_pawn_ref))
  (bind _outoverlappingcomponents (Class|PrimitiveComponent|GetOverlappingComponents _lefthandcollider))
  (bind _outoverlappingcomponents_2 (Class|PrimitiveComponent|GetOverlappingComponents _righthandcollider))
  (if (Variables|Default|GetSpinning)
    (if (or (> (Utilities|Array|Length _outoverlappingcomponents_2) 0) (> (Utilities|Array|Length _outoverlappingcomponents) 0))
      (bind _array_element (Utilities|Array|ForEachLoopwithBreak _outoverlappingcomponents_2 :!label _label)
        (:LoopBody
          (if (Utilities|IsValid _array_element)
            (if (Components|ComponentHasTag _array_element "DrillColliderTag")
              (goto _label Break))))
        (:Completed
          (if (Components|ComponentHasTag _array_element "DrillColliderTag")
            (Utilities|FlowControl|DoOnce false :!label _label_2
              (:Completed
                (Audio|PlaySound2D "/Game/Audio/drill.drill" 0.5 1.0 0.0 0 0 false)
                (Utilities|FlowControl|Delay 0.1)
                (goto _label_2 Reset)))
            (else
              (bind _array_element_2 (Utilities|Array|ForEachLoopwithBreak _outoverlappingcomponents :!label _label_3)
                (:LoopBody
                  (if (Utilities|IsValid _array_element_2)
                    (if (Components|ComponentHasTag _array_element_2 "DrillColliderTag")
                      (goto _label_3 Break))))
                (:Completed
                  (if (Components|ComponentHasTag _array_element_2 "DrillColliderTag")
                    (goto _label_2)))))))))))

(fn ConstructionScript)