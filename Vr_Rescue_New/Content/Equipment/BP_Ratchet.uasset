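; BP_Ratchet is a grabbable ratchet that snaps onto a BP_Rotor anchor point once that rotor has its rope attached.
; On sphere overlap it releases the grab, disables gravity, zeroes velocities, moves to the rotor's RachetPoint, copies only the rotor's yaw and sets IsOnAnchor.
; A DoOnce prevents repeat snapping until the rotor's end overlap resets it, restores gravity and clears IsOnAnchor.
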(event OnComponentBeginOverlap(Sphere)
  (params (OverlappedComponent :type Primitive%20Component%20Object%20Reference) (OtherActor :type Actor%20Object%20Reference) (OtherComp :type Primitive%20Component%20Object%20Reference) (OtherBodyIndex :type Integer) (bFromSweep :type Boolean) (SweepResult :type Hit%20Result%20Structure%20%28by%20ref%29))
  (bind _ratchetmesh (Variables|Default|GetRatchetMesh))
  (bind _asbp_rotor (Utilities|Casting|CastToBP_Rotor OtherActor))
  (if (Variables|/Game/Equipment/BP_Rotor.BP_Rotor_C|GetRopeAttached _asbp_rotor)
    (Utilities|FlowControl|DoOnce false
      (:Completed
        (Default|TryRelease (Variables|Default|GetGrabComponent))
        (Physics|SetEnableGravity _ratchetmesh false)
        (Physics|SetPhysicsLinearVelocity _ratchetmesh "0, 0, 0" false "None")
        (Class|PrimitiveComponent|SetPhysicsAngularVelocityinDegrees _ratchetmesh "0, 0, 0" false "None")
        (Transformation|SetWorldLocation _ratchetmesh (Transformation|GetWorldLocation (Variables|/Game/Equipment/BP_Rotor.BP_Rotor_C|GetRachetPoint _asbp_rotor)) false false)
        (Transformation|SetWorldRotation _ratchetmesh (Math|Rotator|MakeRotator 0.0 0.0 (.yaw (Transformation|GetWorldRotation (Variables|/Game/Equipment/BP_Rotor.BP_Rotor_C|GetRotorMesh _asbp_rotor)))) false false)
        (Variables|Default|SetIsOnAnchor true)))))

(event OnComponentEndOverlap(Sphere)
  (params (OverlappedComponent :type Primitive%20Component%20Object%20Reference) (OtherActor :type Actor%20Object%20Reference) (OtherComp :type Primitive%20Component%20Object%20Reference) (OtherBodyIndex :type Integer))
  (bind _ratchetmesh (Variables|Default|GetRatchetMesh))
  (Utilities|Casting|CastToBP_Rotor OtherActor)
  (Physics|SetEnableGravity (Variables|Default|GetRatchetMesh) true)
  (Variables|Default|SetIsOnAnchor false)
  (Utilities|FlowControl|DoOnce false) ; enters at Reset
)

(event EventBeginPlay)

(event Collision|EventActorBeginOverlap
  (params (OtherActor :type Actor%20Object%20Reference)))

(fn ConstructionScript)