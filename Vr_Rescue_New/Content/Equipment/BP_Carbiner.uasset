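; BP_Carbiner is a grabbable carabiner/descender piece that snaps onto a BP_Anchor when its sphere overlaps one.
; On attach, it releases the grab, plays a clip sound, disables gravity, zeroes velocities and moves the descender body to the anchor's sphere, matching only its yaw.
; A DoOnce prevents repeated snapping; ending the anchor overlap restores gravity, clears IsAttached and re-arms it.
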(event OnComponentBeginOverlap(Sphere)
  (params (OverlappedComponent :type Primitive%20Component%20Object%20Reference) (OtherActor :type Actor%20Object%20Reference) (OtherComp :type Primitive%20Component%20Object%20Reference) (OtherBodyIndex :type Integer) (bFromSweep :type Boolean) (SweepResult :type Hit%20Result%20Structure%20%28by%20ref%29))
  (bind _vr_descenderasset_descender_body (Variables|Default|GetVR_DescenderAsset_Descender_Body))
  (bind _asbp_anchor (Utilities|Casting|CastToBP_Anchor OtherActor))
  (Utilities|FlowControl|DoOnce false
    (:Completed
      (Default|TryRelease (Variables|Default|GetGrabComponent))
      (Audio|PlaySound2D "/Game/Audio/399926__kinoton__carabiner-attach-to-harness-_AudioTrimmer_com_.399926__kinoton__carabiner-attach-to-harness-_AudioTrimmer_com_" 1.0 1.0 0.0 0 0)
      (Physics|SetEnableGravity _vr_descenderasset_descender_body false)
      (Physics|SetPhysicsLinearVelocity _vr_descenderasset_descender_body "0, 0, 0" false "None")
      (Class|PrimitiveComponent|SetPhysicsAngularVelocityinDegrees _vr_descenderasset_descender_body "0, 0, 0" false "None")
      (Transformation|SetWorldLocation _vr_descenderasset_descender_body (Transformation|GetWorldLocation (Variables|/Game/Equipment/BP_Anchor.BP_Anchor_C|GetSphere _asbp_anchor)) false false)
      (Transformation|SetWorldRotation _vr_descenderasset_descender_body (Math|Rotator|MakeRotator 0.0 0.0 (.yaw (Transformation|GetWorldRotation (Variables|/Game/Equipment/BP_Anchor.BP_Anchor_C|GetDefaultSceneRoot _asbp_anchor)))) false false)
      (Variables|Default|SetisAttached true))))

(event OnComponentEndOverlap(Sphere)
  (params (OverlappedComponent :type Primitive%20Component%20Object%20Reference) (OtherActor :type Actor%20Object%20Reference) (OtherComp :type Primitive%20Component%20Object%20Reference) (OtherBodyIndex :type Integer))
  (bind _vr_descenderasset_descender_body (Variables|Default|GetVR_DescenderAsset_Descender_Body))
  (Utilities|Casting|CastToBP_Anchor OtherActor)
  (Physics|SetEnableGravity (Variables|Default|GetVR_DescenderAsset_Descender_Body) true)
  (Variables|Default|SetisAttached false)
  (Utilities|FlowControl|DoOnce false) ; enters at Reset
)

(fn ConstructionScript)