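; Trigger volume that respawns climbing equipment the VR player is not wearing at the upper spawn points.
; When a VRPawn enters the box, it checks the equipped flags for the ratchet, rope bag, rotor and cable clip.
; Each unequipped item's mesh, found by GetActorOfClass, moves to its matching spawn actor and has gravity enabled.
; A DoOnce limits this to once per entry and resets when the pawn leaves.
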(event OnComponentBeginOverlap(Box)
  (params (OverlappedComponent :type Primitive%20Component%20Object%20Reference) (OtherActor :type Actor%20Object%20Reference) (OtherComp :type Primitive%20Component%20Object%20Reference) (OtherBodyIndex :type Integer) (bFromSweep :type Boolean) (SweepResult :type Hit%20Result%20Structure%20%28by%20ref%29))
  (bind _asvrpawn (Utilities|Casting|CastToVRPawn OtherActor))
  (Utilities|FlowControl|DoOnce false
    (:Completed
      (Utilities|FlowControl|Sequence
        (:then_0
          (if (not (Variables|/Game/VRTemplate/Blueprints/VRPawn.VRPawn_C|GetRatchetEquipped _asvrpawn))
            (bind _returnvalue (Actor|GetActorOfClass "/Game/Equipment/BP_Ratchet.BP_Ratchet_C"))
            (bind _returnvalue_2 (Actor|GetActorOfClass "/Game/Equipment/RatchetUpperSpawn.RatchetUpperSpawn_C"))
            (Transformation|SetWorldLocation (Variables|/Game/Equipment/BP_Ratchet.BP_Ratchet_C|GetRatchetMesh _returnvalue) (.location (Transformation|GetActorTransform _returnvalue_2)) false false)
            (Physics|SetEnableGravity (Variables|/Game/Equipment/BP_Ratchet.BP_Ratchet_C|GetRatchetMesh _returnvalue) true)))
        (:then_1
          (if (not (Variables|/Game/VRTemplate/Blueprints/VRPawn.VRPawn_C|GetRopeBagEquipped _asvrpawn))
            (bind _returnvalue_3 (Actor|GetActorOfClass "/Game/Equipment/BP_RopeBag.BP_RopeBag_C"))
            (bind _returnvalue_4 (Actor|GetActorOfClass "/Game/Equipment/RopeBagUpperSpawn.RopeBagUpperSpawn_C"))
            (Transformation|SetWorldLocation (Variables|/Game/Equipment/BP_RopeBag.BP_RopeBag_C|GetVR_Ropebag _returnvalue_3) (.location (Transformation|GetActorTransform _returnvalue_4)) false false)
            (Physics|SetEnableGravity (Variables|/Game/Equipment/BP_RopeBag.BP_RopeBag_C|GetVR_Ropebag _returnvalue_3) true)))
        (:then_2
          (if (not (Variables|/Game/VRTemplate/Blueprints/VRPawn.VRPawn_C|GetRotorEquipped _asvrpawn))
            (bind _returnvalue_5 (Actor|GetActorOfClass "/Game/Equipment/BP_Rotor.BP_Rotor_C"))
            (bind _returnvalue_6 (Actor|GetActorOfClass "/Game/Equipment/PulleyUpperSpawn.PulleyUpperSpawn_C"))
            (Transformation|SetWorldLocation (Variables|/Game/Equipment/BP_Rotor.BP_Rotor_C|GetRotorMesh _returnvalue_5) (.location (Transformation|GetActorTransform _returnvalue_6)) false false)
            (Physics|SetEnableGravity (Variables|/Game/Equipment/BP_Rotor.BP_Rotor_C|GetRotorMesh _returnvalue_5) true)))
        (:then_3
          (if (not (Variables|/Game/VRTemplate/Blueprints/VRPawn.VRPawn_C|GetCableClipEquipped _asvrpawn))
            (bind _returnvalue_7 (Actor|GetActorOfClass "/Game/Equipment/BP_CableClip.BP_CableClip_C"))
            (bind _returnvalue_8 (Actor|GetActorOfClass "/Game/Equipment/CableClipUpperSpawn.CableClipUpperSpawn_C"))
            (Transformation|SetWorldLocation (Variables|/Game/Equipment/BP_CableClip.BP_CableClip_C|GetVR_DescenderAsset_Descender_Body _returnvalue_7) (.location (Transformation|GetActorTransform _returnvalue_8)) false false)
            (Physics|SetEnableGravity (Variables|/Game/Equipment/BP_CableClip.BP_CableClip_C|GetVR_DescenderAsset_Descender_Body _returnvalue_7) true)))))))

(event OnComponentEndOverlap(Box)
  (params (OverlappedComponent :type Primitive%20Component%20Object%20Reference) (OtherActor :type Actor%20Object%20Reference) (OtherComp :type Primitive%20Component%20Object%20Reference) (OtherBodyIndex :type Integer))
  (Utilities|Casting|CastToVRPawn OtherActor)
  (Utilities|FlowControl|DoOnce false) ; enters at Reset
)

(fn ConstructionScript)