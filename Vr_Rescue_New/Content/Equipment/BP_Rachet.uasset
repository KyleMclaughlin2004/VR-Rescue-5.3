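; BP_Rachet is a grabbable VR descender device that snaps onto an attached BP_Carbiner.
; On sphere overlap, a DoOnce releases the grab, disables gravity, zeroes velocities, then teleports the body to the carabiner's RachetPoint with matching yaw only.
; It tracks this state in IsOnAnchor.
; When a carabiner leaves the sphere, it restores gravity, clears IsOnAnchor and resets the DoOnce.
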(event OnComponentBeginOverlap(Sphere)
  (params (OverlappedComponent :type Primitive%20Component%20Object%20Reference) (OtherActor :type Actor%20Object%20Reference) (OtherComp :type Primitive%20Component%20Object%20Reference) (OtherBodyIndex :type Integer) (bFromSweep :type Boolean) (SweepResult :type Hit%20Result%20Structure%20%28by%20ref%29))
  (bind _vr_descenderasset_descender_body (Variables|Default|GetVR_DescenderAsset_Descender_Body))
  (bind _asbp_carbiner (Utilities|Casting|CastToBP_Carbiner OtherActor))
  (if (Variables|/Game/Equipment/BP_Carbiner.BP_Carbiner_C|GetisAttached _asbp_carbiner)
    (Utilities|FlowControl|DoOnce false
      (:Completed
        (Default|TryRelease (Variables|Default|GetGrabComponent))
        (Physics|SetEnableGravity _vr_descenderasset_descender_body false)
        (Physics|SetPhysicsLinearVelocity _vr_descenderasset_descender_body "0, 0, 0" false "None")
        (Class|PrimitiveComponent|SetPhysicsAngularVelocityinDegrees _vr_descenderasset_descender_body "0, 0, 0" false "None")
        (Transformation|SetWorldLocation _vr_descenderasset_descender_body (Transformation|GetWorldLocation (Variables|/Game/Equipment/BP_Carbiner.BP_Carbiner_C|GetRachetPoint _asbp_carbiner)) false false)
        (Transformation|SetWorldRotation _vr_descenderasset_descender_body (Math|Rotator|MakeRotator 0.0 0.0 (.yaw (Transformation|GetWorldRotation (Variables|/Game/Equipment/BP_Carbiner.BP_Carbiner_C|GetDefaultSceneRoot _asbp_carbiner)))) false false)
        (Variables|Default|SetIsOnAnchor true)))))

(event OnComponentEndOverlap(Sphere)
  (params (OverlappedComponent :type Primitive%20Component%20Object%20Reference) (OtherActor :type Actor%20Object%20Reference) (OtherComp :type Primitive%20Component%20Object%20Reference) (OtherBodyIndex :type Integer))
  (bind _vr_descenderasset_descender_body (Variables|Default|GetVR_DescenderAsset_Descender_Body))
  (Utilities|Casting|CastToBP_Carbiner OtherActor)
  (Physics|SetEnableGravity (Variables|Default|GetVR_DescenderAsset_Descender_Body) true)
  (Variables|Default|SetIsOnAnchor false)
  (Utilities|FlowControl|DoOnce false) ; enters at Reset
)

(event EventBeginPlay)

(event Collision|EventActorBeginOverlap
  (params (OtherActor :type Actor%20Object%20Reference)))

(fn ConstructionScript)