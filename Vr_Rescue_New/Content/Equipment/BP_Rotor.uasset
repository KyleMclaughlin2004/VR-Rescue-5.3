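; BP_Rotor is a grabbable physics rotor that snaps onto a BP_Anchor's pulley attach point.
; On sphere overlap with an anchor, a DoOnce releases the grab, plays a carabiner sound, stops motion and gravity, aligns the mesh and switches collision responses to overlap.
; Ending the overlap restores gravity and blocking collision and resets the DoOnce.
; While attached, Tick prints the rotor's location for debugging.
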(event OnComponentBeginOverlap(Sphere)
  (params (OverlappedComponent :type Primitive%20Component%20Object%20Reference) (OtherActor :type Actor%20Object%20Reference) (OtherComp :type Primitive%20Component%20Object%20Reference) (OtherBodyIndex :type Integer) (bFromSweep :type Boolean) (SweepResult :type Hit%20Result%20Structure%20%28by%20ref%29))
  (bind _rotormesh (Variables|Default|GetRotorMesh))
  (bind _asbp_anchor (Utilities|Casting|CastToBP_Anchor OtherActor))
  (Utilities|FlowControl|DoOnce false
    (:Completed
      (Default|TryRelease (Variables|Default|GetGrabComponent))
      (Audio|PlaySound2D "/Game/Audio/399926__kinoton__carabiner-attach-to-harness-_AudioTrimmer_com_.399926__kinoton__carabiner-attach-to-harness-_AudioTrimmer_com_" 1.0 1.0 0.0 0 0)
      (Physics|SetEnableGravity _rotormesh false)
      (Physics|SetPhysicsLinearVelocity _rotormesh "0, 0, 0" false "None")
      (Class|PrimitiveComponent|SetPhysicsAngularVelocityinDegrees _rotormesh "0, 0, 0" false "None")
      (Transformation|SetWorldLocation _rotormesh (Transformation|GetWorldLocation (Variables|/Game/Equipment/BP_Anchor.BP_Anchor_C|GetPulleyAttachPoint _asbp_anchor)) false false)
      (Transformation|SetWorldRotation _rotormesh (Math|Rotator|MakeRotator 0.0 0.0 (.yaw (Transformation|GetWorldRotation (Variables|/Game/Equipment/BP_Anchor.BP_Anchor_C|GetDefaultSceneRoot _asbp_anchor)))) false false)
      (Transformation|SetWorldRotation (Variables|Default|GetScene) (Math|Rotator|MakeRotator 0.0 0.0 (+ 0.0 9e+01)) false false)
      (Variables|Default|SetIsAttached true)
      (Collision|SetCollisionResponsetoChannel _rotormesh "ECC_WorldStatic" "ECR_Overlap")
      (Collision|SetCollisionResponsetoChannel _rotormesh "ECC_Pawn" "ECR_Overlap")
      (Collision|SetCollisionResponsetoChannel _rotormesh "ECC_PhysicsBody" "ECR_Overlap")
      (Collision|SetCollisionResponsetoChannel _rotormesh "ECC_WorldDynamic" "ECR_Overlap"))))

(event OnComponentEndOverlap(Sphere)
  (params (OverlappedComponent :type Primitive%20Component%20Object%20Reference) (OtherActor :type Actor%20Object%20Reference) (OtherComp :type Primitive%20Component%20Object%20Reference) (OtherBodyIndex :type Integer))
  (bind _rotormesh (Variables|Default|GetRotorMesh))
  (bind _rotormesh_2 (Variables|Default|GetRotorMesh))
  (Utilities|Casting|CastToBP_Anchor OtherActor)
  (Physics|SetEnableGravity _rotormesh_2 true)
  (Variables|Default|SetIsAttached false)
  (Collision|SetCollisionResponsetoChannel _rotormesh_2 "ECC_WorldStatic" "ECR_Block")
  (Collision|SetCollisionResponsetoChannel _rotormesh_2 "ECC_Pawn" "ECR_Block")
  (Collision|SetCollisionResponsetoChannel _rotormesh_2 "ECC_PhysicsBody" "ECR_Block")
  (Collision|SetCollisionResponsetoChannel _rotormesh_2 "ECC_WorldDynamic" "ECR_Block")
  (Utilities|FlowControl|DoOnce false) ; enters at Reset
)

(event EventBeginPlay
  (Physics|SetEnableGravity (Variables|Default|GetRotorMesh) true))

(event EventTick
  (params (DeltaSeconds :type Float%20%28single-precision%29))
  ;[1 1 1] DEBUG STUFF TO PRINT ROTOR LOCATION
  (if (Variables|Default|GetIsAttached)
    (Development|PrintString (Utilities|String|ToString(Vector) (Transformation|GetWorldLocation (Variables|Default|GetRotorMesh))))))

(fn ConstructionScript)