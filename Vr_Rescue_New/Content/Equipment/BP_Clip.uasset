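; BP_Clip is a grabbable rope clip that snaps onto a BP_DummyTest when its sphere overlaps that actor.
; On overlap it releases the grab, disables gravity, zeroes velocities, moves to the dummy's sphere and matches the harness yaw.
; It holds without attachment or constraint, tracking state in AttachedToDummy.
; A DoOnce prevents repeat snapping until end overlap restores gravity and resets it.
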(event OnComponentBeginOverlap(Sphere)
  (params (OverlappedComponent :type Primitive%20Component%20Object%20Reference) (OtherActor :type Actor%20Object%20Reference) (OtherComp :type Primitive%20Component%20Object%20Reference) (OtherBodyIndex :type Integer) (bFromSweep :type Boolean) (SweepResult :type Hit%20Result%20Structure%20%28by%20ref%29))
  (bind _ropeclipmesh (Variables|Default|GetRopeClipMesh))
  (bind _asbp_dummy_test (Utilities|Casting|CastToBP_DummyTest OtherActor))
  (Utilities|FlowControl|DoOnce false
    (:Completed
      (Default|TryRelease (Variables|Default|GetGrabComponent))
      (Physics|SetEnableGravity _ropeclipmesh false)
      (Physics|SetPhysicsLinearVelocity _ropeclipmesh "0, 0, 0" false "None")
      (Class|PrimitiveComponent|SetPhysicsAngularVelocityinDegrees _ropeclipmesh "0, 0, 0" false "None")
      (Transformation|SetWorldLocation _ropeclipmesh (Transformation|GetWorldLocation (Variables|/Game/BP_DummyTest.BP_DummyTest_C|GetSphere _asbp_dummy_test)) false false)
      (Transformation|SetWorldRotation _ropeclipmesh (Math|Rotator|MakeRotator 0.0 0.0 (.yaw (Transformation|GetWorldRotation (Variables|/Game/BP_DummyTest.BP_DummyTest_C|GetHarness1 _asbp_dummy_test)))) false false)
      (Variables|Default|SetAttachedToDummy true))))

(event OnComponentEndOverlap(Sphere)
  (params (OverlappedComponent :type Primitive%20Component%20Object%20Reference) (OtherActor :type Actor%20Object%20Reference) (OtherComp :type Primitive%20Component%20Object%20Reference) (OtherBodyIndex :type Integer))
  (bind _ropeclipmesh (Variables|Default|GetRopeClipMesh))
  (Utilities|Casting|CastToBP_DummyTest OtherActor)
  (Physics|SetEnableGravity (Variables|Default|GetRopeClipMesh) true)
  (Variables|Default|SetAttachedToDummy false)
  (Utilities|FlowControl|DoOnce false) ; enters at Reset
)

(fn ConstructionScript)